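; Chasm audio actor that keeps a sound at the point on a spline nearest the first-person player character.
; BeginPlay caches the character, then MoveAudio moves the Audio and Arrow components to that closest point, raised slightly on Z.
; MoveAudio re-calls itself after a short Delay instead of using Tick, and the loop ends if the character reference becomes invalid.
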(event `self.ReceiveBeginPlay`
  (bind _asbp_first_person_character (cast `/Game/Necropolis/Demo/Character/Blueprints/BP_FirstPersonCharacter` (`GameplayStatics.GetPlayerCharacter` 0)))
  (set `self.CharRef` _asbp_first_person_character)
  (`self.Move Audio`))

(event `Move Audio`
  (bind _charref (`self.CharRef`))
  (bind (_returnvalue_x _returnvalue_y _returnvalue_z) (`KismetMathLibrary.BreakVector` (`SplineComponent.FindLocationClosestToWorldLocation` (`self.Spline`) (`self.K2_GetActorLocation` _charref) "World")))
  (`/Engine/EditorBlueprintResources/StandardMacros.IsValid` _charref
    (:`Is Valid`
      (`SceneComponent.K2_SetWorldLocation` (`self.Audio`) (`KismetMathLibrary.MakeVector` _returnvalue_x _returnvalue_y (+ _returnvalue_z 50.0)) false false)
      (`SceneComponent.K2_SetWorldLocation` (`self.Arrow`) (`KismetMathLibrary.MakeVector` _returnvalue_x _returnvalue_y (+ _returnvalue_z 50.0)) false false)
      (`KismetSystemLibrary.Delay` 0.4)
      (`self.Move Audio`))))

(fn `UserConstructionScript`)