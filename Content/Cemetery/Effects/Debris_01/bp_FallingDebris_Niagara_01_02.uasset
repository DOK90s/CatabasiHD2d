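; Falling debris effect actor that intermittently fires a Niagara system alongside a DirtDebris component, likely audio.
; The construction script assigns the chosen Niagara asset to the component.
; From BeginPlay, an endless loop waits a random delay, activates both components for a random duration, then deactivates the particles.
; DirtDebris stops one second after the particles, while the next delay is already running.
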(event `self.ReceiveBeginPlay`
  (bind _niagarasystem (`self.NiagaraSystem`))
  (`/Engine/EditorBlueprintResources/StandardMacros.IsValid` (`self.Niagara`)
    (:`Is Valid`
      (`ActorComponent.SetAutoActivate` _niagarasystem false)
      (`ActorComponent.Deactivate` _niagarasystem)
      (`KismetSystemLibrary.Delay` (`KismetMathLibrary.RandomFloatInRange` (`self.DelayMin`) (`self.DelayMax`)) :!label _label)
      (`ActorComponent.Activate` (`self.NiagaraSystem`) false)
      (`AudioComponent.Play` (`self.Dirt_Debris`) 0.0)
      (`KismetSystemLibrary.Delay` (`KismetMathLibrary.RandomFloatInRange` (`self.DurationMin`) (`self.DurationMax`)))
      (`ActorComponent.Deactivate` (`self.NiagaraSystem`))
      (`|ExecutionSequence`
        (:`then_0`
          (goto _label))
        (:`then_1`
          (`KismetSystemLibrary.Delay` 1.0)
          (`AudioComponent.Stop` (`self.Dirt_Debris`)))))))

(fn `UserConstructionScript`
  (bind _niagara (`self.Niagara`))
  (`/Engine/EditorBlueprintResources/StandardMacros.IsValid` _niagara
    (:`Is Valid`
      (`NiagaraComponent.SetAsset` (`self.NiagaraSystem`) _niagara true))))