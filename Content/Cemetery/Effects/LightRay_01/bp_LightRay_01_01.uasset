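; Light ray effect actor for the cemetery environment, configurable per placed instance.
; The construction script creates a dynamic material from a base material on the LightRay component's first slot.
; It then pushes the exposed color, depth fade opacity, fade distance and fade offset variables into that material.
; The event graph holds only disabled stub events, so all setup happens at construction.
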(fn `UserConstructionScript`
  (bind _materialdynamic (`self.MaterialDynamic`))
  (bind _returnvalue (`PrimitiveComponent.CreateDynamicMaterialInstance` (`self.LightRay`) 0 (`self.MaterialBase`) "None"))
  (set `self.MaterialDynamic` _returnvalue)
  (`MaterialInstanceDynamic.SetScalarParameterValue` _materialdynamic "Depth Fade Opacity" (`self.DepthFadeOpacity`))
  (`MaterialInstanceDynamic.SetScalarParameterValue` _materialdynamic "Fade Distance" (`self.FadeDistance`))
  (`MaterialInstanceDynamic.SetVectorParameterValue` _materialdynamic "Color" (`self.Color`))
  (`MaterialInstanceDynamic.SetScalarParameterValue` _materialdynamic "Fade Offset" (`self.FadeOffset`)))