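; Chain spline actor for the cemetery chandelier set that builds a chain from repeated link meshes along an editable spline.
; The construction script fills a hierarchical instanced static mesh, spacing links by scaled mesh length minus offset, with a default mesh fallback.
; Each link aims at the next spline point, with alternate links rolled 90 degrees to interlock and an adjustable progressive twist along the length.
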(fn `UserConstructionScript`
  (bind _sectionoffset (`self.SectionOffset`))
  (bind _scale (`self.Scale`))
  (bind _hierarchicalinstancedstaticmesh (`self.HierarchicalInstancedStaticMesh`))
  (bind _spline (`self.Spline`))
  (bind _sectionlength (`self.SectionLength`))
  (bind _staticmesh (`self.StaticMesh`)
    (:`then`
      (`StaticMeshComponent.SetStaticMesh` _hierarchicalinstancedstaticmesh _staticmesh))
    (:`else`
      (`StaticMeshComponent.SetStaticMesh` _hierarchicalinstancedstaticmesh "/Game/Cemetery/Environment/Chandelier_01/sm_Chandelier_01_02.sm_Chandelier_01_02")))
  (set `self.SectionLength` (* (`self.MeshLength`) _scale))
  (set `self.SectionOffset` (* (`self.MeshOffset`) _scale))
  (for _index (range (`KismetMathLibrary.FTrunc` (/ (`SplineComponent.GetSplineLength` (`self.Spline`)) (- (`self.SectionLength`) (`self.SectionOffset`)))))
    (bind _returnvalue (- (* _index _sectionlength) (* _index _sectionoffset)))
    (bind _returnvalue_2 (`SplineComponent.GetLocationAtDistanceAlongSpline` _spline _returnvalue "Local"))
    (bind _returnvalue_3 (* (/ _returnvalue (`self.RotationSegmentLength`)) (`self.RotationAmount`)))
    (bind _returnvalue_4 (+ _index 1))
    (bind _pitch (.pitch (`KismetMathLibrary.FindLookAtRotation` _returnvalue_2 (`SplineComponent.GetLocationAtDistanceAlongSpline` _spline (- (* _returnvalue_4 _sectionlength) (* _returnvalue_4 _sectionoffset)) "Local"))))
    (bind _yaw (.yaw (`KismetMathLibrary.FindLookAtRotation` _returnvalue_2 (`SplineComponent.GetLocationAtDistanceAlongSpline` _spline (- (* _returnvalue_4 _sectionlength) (* _returnvalue_4 _sectionoffset)) "Local"))))
    (`InstancedStaticMeshComponent.AddInstance` (`self.HierarchicalInstancedStaticMesh`) (`KismetMathLibrary.MakeTransform` _returnvalue_2 (`KismetMathLibrary.SelectRotator` (`KismetMathLibrary.MakeRotator` _returnvalue_3 _pitch _yaw) (`KismetMathLibrary.MakeRotator` (+ _returnvalue_3 90.0) _pitch _yaw) (not (`KismetMathLibrary.Conv_IntToBool` (mod _index 2)))) (`KismetMathLibrary.Conv_DoubleToVector` (`self.Scale`))) false)))